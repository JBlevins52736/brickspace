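; Player state for a colocation session, relaying spatial-anchor alignment, share notifications and cube spawning over the network.
; Server_OrientToAnchor teleports the player's pawn to the given position and rotation, then multicasts that transform so every client applies it.
; Server_spawnCube spawns a quarter-scale BP_2x5 at the requested position.
; Server_NotifyShare multicasts LoadShared, whose handler is empty; the anchor lookup and orient nodes are left unconnected.
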(event `self.ReceiveBeginPlay`)

(event `server_spawnCube`
  (params (Position :type "Vector Structure"))
  (`|SpawnActorFromClass` "/Game/Blueprints/BP_2x5.BP_2x5_C" (`KismetMathLibrary.MakeTransform` Position (struct) (0.25 0.25 0.25)) "Undefined" "OverrideRootScale" null null))

(event `Server_OrientToAnchor`
  (params (Position :type "Vector Structure") (Rotation :type "Rotator Structure"))
  (bind _pawnprivate (`self.PawnPrivate`))
  (`self.K2_SetActorLocation` _pawnprivate Position false true)
  (`self.K2_SetActorRotation` _pawnprivate Rotation true)
  (`self.NetMulticast_setPosition` Position Rotation))

(event `NetMulticast_setPosition`
  (params (Position :type "Vector Structure") (Rotation :type "Rotator Structure"))
  (bind _pawnprivate (`self.PawnPrivate`))
  (`self.K2_SetActorLocation` _pawnprivate Position false true)
  (`self.K2_SetActorRotation` _pawnprivate Rotation true))

(event `Server_NotifyShare`
  (`self.NetMulticast_loadShared`))

(event `NetMulticast_LoadShared`)

(fn `UserConstructionScript`)