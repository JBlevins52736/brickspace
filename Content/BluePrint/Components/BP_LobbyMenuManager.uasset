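; Lobby menu manager that spawns a BP_Lobby_Menu at the MainMenuPositioner transform and routes menu input to it.
; On BeginPlay it passes SessionManager to the new menu, stores it as the current menu context and hands that context back to SessionManager.
; Selection and up/down events forward to the menu, while Tick keeps it locked to the positioner.
; An Android storage-permission check is present but disconnected.
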(event `self.ReceiveBeginPlay`
  ; Main Menu Setup
  (bind _returnvalue (`|SpawnActorFromClass` "/Game/BluePrint/UI/BP_Lobby_Menu.BP_Lobby_Menu_C" (`SceneComponent.K2_GetComponentToWorld` (`self.MainMenuPositioner`)) "Undefined" "MultiplyWithRoot" null (`self.Session Manager`) null null))
  (bind _output_get (set `self.MainMenu` _returnvalue))
  (bind _output_get_2 (set `self.CurrentMenuContext` _output_get))
  (set `/Game/BP_SessionManager.Menu` _output_get_2 (`self.Session Manager`)))

(event `Select Main Menu Item`
  (bind _mainmenu (`self.MainMenu`))
  (`/Engine/EditorBlueprintResources/StandardMacros.IsValid` _mainmenu
    (:`Is Valid`
      (`/Game/BluePrint/UI/BP_Menu.Run Select` _mainmenu))))

(event `Select Menu Item`
  (`/Game/BluePrint/UI/BP_Menu.Run Select` (`self.CurrentMenuContext`)))

(event `self.ReceiveTick`
  (params (DeltaSeconds :type "Float (single-precision)"))
  (bind _mainmenu (`self.MainMenu`))
  (`/Engine/EditorBlueprintResources/StandardMacros.IsValid` _mainmenu
    (:`Is Valid`
      (`Actor.K2_SetActorTransform` _mainmenu (`SceneComponent.K2_GetComponentToWorld` (`self.MainMenuPositioner`)) false false))))

(event `Menu Selection Up`
  (`/Game/BluePrint/UI/BP_Menu.Menu Selection Up` (`self.CurrentMenuContext`)))

(event `Menu selection down`
  (`/Game/BluePrint/UI/BP_Menu.Menu Selection Down` (`self.CurrentMenuContext`)))