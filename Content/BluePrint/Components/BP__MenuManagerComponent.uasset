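; Pawn component that manages spatial-anchor menus for the locally controlled player and forwards navigation and select input to the current menu context.
; After a startup delay it spawns the main menu, which follows a positioner every Tick.
; SpatialAnchorManager dispatchers switch context between anchor and main menus.
; ReturnAnchorMenu destroys any existing anchor menu, but its spawn-and-attach chain is unreachable, so no replacement appears.
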(event `select main menu item`
  (bind _mainmenu (`self.MainMenu`))
  (`/Engine/EditorBlueprintResources/StandardMacros.IsValid` _mainmenu
    (:`Is Valid`
      (`/Game/BluePrint/UI/BP_Menu.Run Select` _mainmenu))))

(event `Menu Selection up`
  (`/Game/BluePrint/UI/BP_Menu.Menu Selection Up` (`self.CurrentMenuContext`)))

(event `Select menu item`
  (`/Game/BluePrint/UI/BP_Menu.Run Select` (`self.CurrentMenuContext`)))

(event `Menu Seelection down`
  (`/Game/BluePrint/UI/BP_Menu.Menu Selection Down` (`self.CurrentMenuContext`)))

(event `Select Anchor Menu Item`
  (bind _anchor_menu (`self.Anchor Menu`))
  (`/Engine/EditorBlueprintResources/StandardMacros.IsValid` _anchor_menu
    (:`Is Valid`
      (`/Game/BluePrint/UI/BP_Menu.Run Select` _anchor_menu))))

(event `self.ReceiveBeginPlay`
  (bind _spatialanchormanager (`self.SpatialAnchorManager`))
  (`KismetSystemLibrary.Delay` 2.0)
  (bind _aspawn (cast `Pawn` (`self.GetOwner`)))
  (if (`Pawn.IsLocallyControlled` _aspawn)
    (`|ExecutionSequence`
      (:`then_0`
        (bind _returnvalue (`|SpawnActorFromClass` "/Game/BluePrint/UI/Bp_menu_main.Bp_menu_main_C" (`SceneComponent.K2_GetComponentToWorld` (`self.MainMenuPositioner`)) "Undefined" "OverrideRootScale" null null self null (`self.SpatialAnchorManager`) null))
        (bind _output_get (set `self.MainMenu` _returnvalue))
        (set `self.CurrentMenuContext` _output_get)
        (set `/Game/BluePrint/Components/BP_SpatialAnchorManager.MenuManager` self (`self.SpatialAnchorManager`)))
      (:`then_1`
        (`|ExecutionSequence`
          (:`then_0`
            (add `/Game/BluePrint/Components/BP_SpatialAnchorManager.AnchorSavedDispatch` _spatialanchormanager (delegate `Activate Anchor Menu`)))
          (:`then_1`
            (add `/Game/BluePrint/Components/BP_SpatialAnchorManager.AnchorUnsavedDispatch` _spatialanchormanager (delegate `Activate Anchor Menu`)))
          (:`then_2`
            (add `/Game/BluePrint/Components/BP_SpatialAnchorManager.AnchorSelectedDispatch` _spatialanchormanager (delegate `Activate Anchor Menu`)))))
      (:`then_2`
        (add `/Game/BluePrint/Components/BP_SpatialAnchorManager.AnchorUnselectedDispatch` _spatialanchormanager (delegate `Deactivate Anchor Menu`))))))

(event `self.ReceiveTick`
  (params (DeltaSeconds :type "Float (single-precision)"))
  (bind _mainmenu (`self.MainMenu`))
  (bind _aspawn (cast `Pawn` (`self.GetOwner`)))
  (if (`Pawn.IsLocallyControlled` _aspawn)
    (`|ExecutionSequence`
      (:`then_0`
        (`/Engine/EditorBlueprintResources/StandardMacros.IsValid` _mainmenu
          (:`Is Valid`
            (`Actor.K2_SetActorTransform` _mainmenu (`SceneComponent.K2_GetComponentToWorld` (`self.MainMenuPositioner`)) false false))))
      (:`then_1`
        (bind _anchorselected (`/Game/BluePrint/Components/BP_SpatialAnchorManager.HasSelectedAnchor` (`self.SpatialAnchorManager`)))
        (if _anchorselected
          _)))))

(event `Deactivate Anchor Menu`
  (bind _anchor_menu (`self.Anchor Menu`))
  (`/Engine/EditorBlueprintResources/StandardMacros.IsValid` _anchor_menu
    (:`Is Valid`
      (`Actor.K2_DestroyActor` _anchor_menu)
      (set `self.CurrentMenuContext` (`self.MainMenu`)))))

(event `Activate Anchor Menu`
  (bind _anchorselected (`/Game/BluePrint/Components/BP_SpatialAnchorManager.HasSelectedAnchor` (`self.SpatialAnchorManager`)))
  (if _anchorselected
    (bind _anchor_menu (`self.ReturnAnchorMenu` (`self.AnchorMenuPositioner`)))
    (set `self.CurrentMenuContext` _anchor_menu)))

(fn `ReturnAnchorMenu`
  (params (SceneComponentToAttachTo :type "SceneComponent Object Reference"))
  (returns (`Anchor Menu` :type "/Game/BluePrint/UI/BP_menu_Anchor Object Reference"))
  (bind _anchor_menu (`self.Anchor Menu`))
  (`/Engine/EditorBlueprintResources/StandardMacros.IsValid` _anchor_menu
    (:`Is Valid`
      (`Actor.K2_DestroyActor` _anchor_menu))))