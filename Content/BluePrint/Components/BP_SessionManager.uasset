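; Session manager component that hosts and joins Meta Quest colocation multiplayer sessions for the BrickSpace level.
; Hosting creates a session, advertises the local IP as colocation session data, stores it on the game instance and opens BrickSpace as a listen server.
; Joining discovers colocation sessions, saves the found one to the game instance and connects to it.
; Both flows report progress and results to the Menu via StartAsync and EndAsync.
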(event `Create Session`
  ; Create Session
  (`CreateSessionCallbackProxy.CreateSession` (`GameplayStatics.GetPlayerController` 0) 5
    (:`then`
      (`/Game/BluePrint/UI/BP_Menu.Start Async` (`self.Menu`)))
    (:`OnSuccess`
      (bind _returnvalue (`ColocationSetup.CreateByteArrayFromString` (`ColocationSetup.GetLocalIPAsString`)))
      (bind (_success _session) (`OculusXRAsyncAction_StartColocationSessionAdvertisement.OculusXRAsyncStartColocationSessionAdvertisement` _returnvalue)
        (:`OnComplete`
          (if _success
            (`/Game/BluePrint/UI/BP_Menu.End Async` (`self.Menu`) true)
            (bind _asbp_colocation_session_game_instance (cast `/Game/BluePrint/BP_ColocationSessionGameInstance` (`GameplayStatics.GetGameInstance`)))
            (set `/Game/BluePrint/BP_ColocationSessionGameInstance.ColocationSession` _session _asbp_colocation_session_game_instance)
            (`GameplayStatics.OpenLevelBySoftObjectPtr` "/Game/Maps/BrickSpace.BrickSpace" true "?listen")
            (else
              (`/Game/BluePrint/UI/BP_Menu.End Async` (`self.Menu`) false))))))
    (:`OnFailure`
      (`/Game/BluePrint/UI/BP_Menu.End Async` (`self.Menu`) false))))

(event `Find Sessions`
  (bind _menu (`self.Menu`))
  ; Join Session
  (bind (_success _session) (`OculusXRAsyncAction_DiscoverColocationSessions.OculusXRAsyncDiscoverColocationSessions`)
    (:`then`
      (`/Game/BluePrint/UI/BP_Menu.Start Async` _menu))
    (:`SessionFound`
      (bind _asbp_colocation_session_game_instance (cast `/Game/BluePrint/BP_ColocationSessionGameInstance` (`GameplayStatics.GetGameInstance`))
        (:`then`
          (bind _output_get (set `/Game/BluePrint/BP_ColocationSessionGameInstance.ColocationSession` _session _asbp_colocation_session_game_instance))
          (bind _returnvalue (`ColocationSetup.JoinColocationSession` _output_get))
          (`/Game/BluePrint/UI/BP_Menu.End Async` (`self.Menu`) _returnvalue))
        (:`CastFailed`
          (`/Game/BluePrint/UI/BP_Menu.End Async` (`self.Menu`) false))))
    (:`OnComplete`
      (if (not _success)
        (`/Game/BluePrint/UI/BP_Menu.End Async` _menu false)))))