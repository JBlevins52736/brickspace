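; Pawn component that manages Meta Quest spatial anchors for colocated sessions, with a preview model and anchor/cube selection modes.
; Shares selected anchors to the colocation session's group through async OculusXR nodes, reporting to the menu and player state.
; Server requests for cube spawning and anchor orientation go through the owner's player state.
; Unfinished: anchor creation from fetched anchors, saved-anchor restore and cube unhover do nothing.
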(event `self.ReceiveBeginPlay`
  ; Startup- Sets defaults
  (`|ExecutionSequence`
    (:`then_0`
      (`/Game/BluePrint/BP_ColorcationSessionPlayer.Server_OrientToAnchor` :`self` (`self.GetOwningPlayerState`)))
    (:`then_1`
      (bind _returnvalue (`GameplayStatics.LoadGameFromSlot` "SaveGame"))
      (bind _asbp_shared_anchor_save_game (cast `/Game/BluePrint/Components/BP_SharedAnchorSaveGame` _returnvalue))
      (for _ (`/Game/BluePrint/Components/BP_SharedAnchorSaveGame.SavedAnchors` _asbp_shared_anchor_save_game)
        _))))

(event `SpawnCube`
  (cast `/Game/BP_BrickworldPawn` (`GameplayStatics.GetPlayerPawn` 0))
  (`/Game/BluePrint/BP_ColorcationSessionPlayer.server_spawnCube` (`self.GetOwningPlayerState`) (0.0 0.0 0.0)))

(event `OnRecenterHeadset`
  (bind _origin_aanchor (`self.Origin aanchor`))
  (`/Engine/EditorBlueprintResources/StandardMacros.IsValid` _origin_aanchor
    (:`Is Valid`
      (set `self.CachedOriginAnchor` _origin_aanchor))))

(event `ShareAnchors`
  (`KismetArrayLibrary.Array_Clear` (`self.AnchorIDsToShareToLG`))
  (for _array_element (`self.SelectedAnchors`)
    (`KismetArrayLibrary.Array_Add` (`self.AnchorIDsToShareToLG`) (`OculusXRAnchorComponent.GetHandle` (`/Game/BluePrint/BP_SpatialAnchorModel.OculusSpatialAnchor` _array_element))))
  (bind _asbp_colocation_session_game_instance (cast `/Game/BluePrint/BP_ColocationSessionGameInstance` (`GameplayStatics.GetGameInstance`)))
  (`self.StartAsync`)
  (bind _success (`OculusXRAsyncAction_ShareAnchorsWithGroups.OculusXRShareAnchorsWithGroupsAsync` (`|MakeArray` (`.Uuid` (break `OculusXRColocationSession` (`/Game/BluePrint/BP_ColocationSessionGameInstance.ColocationSession` _asbp_colocation_session_game_instance)))) (`self.AnchorIDsToShareToLG`))
    (:`Complete`
      (if _success
        (bind _asbp_colorcation_session_player (cast `/Game/BluePrint/BP_ColorcationSessionPlayer` (`GameplayStatics.GetPlayerState` 0)))
        (`/Game/BluePrint/BP_ColorcationSessionPlayer.Server_NotifyShare` _asbp_colorcation_session_player)
        (`self.EndAsync` _success)))))

(event `GetAllSharedAnchors`
  (bind _asbp_colocation_session_game_instance (cast `/Game/BluePrint/BP_ColocationSessionGameInstance` (`GameplayStatics.GetGameInstance`)))
  (bind (_success _anchors) (`OculusXRAsyncAction_GetSharedAnchorsFromGroup.OculusXRGetSharedAnchorsFromGroupAsync` (`.Uuid` (break `OculusXRColocationSession` (`/Game/BluePrint/BP_ColocationSessionGameInstance.ColocationSession` _asbp_colocation_session_game_instance))))
    (:`Complete`
      (if _success
        (`self.CreateAnchors` _anchors)))))

(event `Activate Model`
  (`/Engine/EditorBlueprintResources/StandardMacros.IsValid` (`self.TempSpatialAnchorModel`)
    (:`Is Not Valid`
      (bind _returnvalue (`|SpawnActorFromClass` "/Game/BluePrint/BP_SpatialAnchorModel.BP_SpatialAnchorModel_C" (`SceneComponent.K2_GetComponentToWorld` (`self.ModelSPawnPositioner`)) "Undefined" "OverrideRootScale" null true null))
      (set `self.TempSpatialAnchorModel` _returnvalue))))

(event `DeactivateModel`
  (bind _tempspatialanchormodel (`self.TempSpatialAnchorModel`))
  (`/Engine/EditorBlueprintResources/StandardMacros.IsValid` _tempspatialanchormodel
    (:`Is Valid`
      (`Actor.K2_DestroyActor` _tempspatialanchormodel)
      (set `self.TempSpatialAnchorModel` null))))

(event `self.ReceiveTick`
  (params (DeltaSeconds :type "Float (single-precision)"))
  (bind _tempspatialanchormodel (`self.TempSpatialAnchorModel`))
  (`|ExecutionSequence`
    (:`then_0`
      (`/Engine/EditorBlueprintResources/StandardMacros.IsValid` _tempspatialanchormodel
        (:`Is Valid`
          (`Actor.K2_SetActorTransform` _tempspatialanchormodel (`SceneComponent.K2_GetComponentToWorld` (`self.ModelSPawnPositioner`)) false false))))))

(event `Enter Anchor Selection Mode`
  (set `self.bAnchorSelectionMode` true))

(event `Exit AnchorSelection Mode`
  (set `self.bAnchorSelectionMode` false)
  (`self.UnsetHoveredAnchor` (`self.Hovered Anchor`)))

(event `Enter Cube Selection Mode`
  (set `self.bCubeSelectionMode` true))

(event `Exit Cube Selection Mode`
  (set `self.bCubeSelectionMode` false)
  (`self.UnsetHoverCube` (`self.Hovered Cube`)))

(fn `CreateAnchorFromUUIDAndHandle`
  (params (UUID :type "OculusXRUUID Structure") (Handle :type "OculusXRUInt64 Structure")))

(fn `createAnchors`
  (params (Anchors :type "Array of OculusXRAnchor Structure"))
  (locals (NewLocalVar :type "OculusXRUUID Structure"))
  (for _array_element Anchors
    (bind (_anchorhandle _uuid) (break `OculusXRAnchor` _array_element))
    (`self.CreateAnchorFromUUIDAndHandle` _uuid _anchorhandle)))

(fn `EndAsync`
  (params (Success :type Boolean))
  (`/Game/BluePrint/UI/BP_Menu.End Async` (`/Game/BluePrint/Components/BP__MenuManagerComponent.CurrentMenuContext` (`self.MenuManager`)) Success))

(fn `FindAnchor`
  (params (UUID :type "OculusXRUUID Structure"))
  (returns (Anchor :type "/Game/BluePrint/BP_SpatialAnchorModel Object Reference"))
  (for _array_element (`self.LoadedAnchors`)
    (if (`OculusXRAnchorBPFunctionLibrary.IsEqual_FOculusXRUUID` (`OculusXRAnchorComponent.GetUUID` (`/Game/BluePrint/BP_SpatialAnchorModel.OculusSpatialAnchor` _array_element)) UUID)
      (return _array_element)))
  (return null))

(fn `GetOwningPlayerState`
  (returns (`Player state` :type "/Game/BluePrint/BP_ColorcationSessionPlayer Object Reference"))
  (bind _aspawn (cast `Pawn` (`self.GetOwner`)))
  (bind _asbp_colorcation_session_player (cast `/Game/BluePrint/BP_ColorcationSessionPlayer` (`Pawn.PlayerState` _aspawn))
    (:`then`
      (return _asbp_colorcation_session_player))
    (:`CastFailed`
      (return null))))

(fn `HasSelectedAnchor`
  (returns (AnchorSelected :type Boolean))
  (return (> (`KismetArrayLibrary.Array_Length` (`self.SelectedAnchors`)) 0)))

(fn `StartAsync`
  (`/Game/BluePrint/UI/BP_Menu.Start Async` (`/Game/BluePrint/Components/BP__MenuManagerComponent.CurrentMenuContext` (`self.MenuManager`))))

(fn `UnsetHoverCube`
  (params (Cube :type "/Game/Blueprints/BP_2x3 Object Reference")))

(fn `UnsetHoveredAnchor`
  (params (`Spatial Anchor` :type "/Game/BluePrint/BP_SpatialAnchorModel Object Reference"))
  (bind _hovered_anchor (`self.Hovered Anchor`))
  (`/Engine/EditorBlueprintResources/StandardMacros.IsValid` `Spatial Anchor`
    (:`Is Valid`
      (if (== `Spatial Anchor` _hovered_anchor)
        (`/Game/BluePrint/BP_SpatialAnchorModel.SetHoveredOnModel` _hovered_anchor false)
        (set `self.Hovered Anchor` null)))))