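; Session manager that creates an online session and advertises it for Meta XR colocation.
; CreateSession makes the session, then starts an OculusXR colocation advertisement carrying the local IP string as a byte array.
; When advertising succeeds, it stores the colocation session in BP_ColocationSessionGameInstance and opens the BrickSpace level.
; The Menu's async state starts with the request and ends on either success or failure.
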(event `Create Session`
  (bind _menu (`self.Menu`))
  (`CreateSessionCallbackProxy.CreateSession` (`GameplayStatics.GetPlayerController` 0) 5
    (:`then`
      (`/Game/BluePrint/UI/BP_Menu.Start Async` _menu))
    (:`OnSuccess`
      (bind _returnvalue (`ColocationSetup.CreateByteArrayFromString` (`ColocationSetup.GetLocalIPAsString`)))
      (bind (_success _session) (`OculusXRAsyncAction_StartColocationSessionAdvertisement.OculusXRAsyncStartColocationSessionAdvertisement` _returnvalue)
        (:`OnComplete`
          (if _success
            (`/Game/BluePrint/UI/BP_Menu.End Async` (`self.Menu`) false)
            (bind _asbp_colocation_session_game_instance (cast `/Game/BluePrint/BP_ColocationSessionGameInstance` (`GameplayStatics.GetGameInstance`)))
            (set `/Game/BluePrint/BP_ColocationSessionGameInstance.ColocationSession` _session _asbp_colocation_session_game_instance)
            (`GameplayStatics.OpenLevelBySoftObjectPtr` "/Game/Maps/BrickSpace.BrickSpace")
            (else
              (`/Game/BluePrint/UI/BP_Menu.End Async` (`self.Menu`) false))))))
    (:`OnFailure`
      (`/Game/BluePrint/UI/BP_Menu.End Async` _menu false))))

(fn `UserConstructionScript`)