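; Session manager that hosts and joins Meta Quest colocation sessions for shared mixed-reality multiplayer, using OculusXR.
; CreateSession creates an online session, advertises a colocation session carrying the local IP as bytes, then opens BrickSpace as a listen server.
; FindSessions discovers advertised colocation sessions and joins each successfully found one.
; Both paths store the colocation session in BP_ColocationSessionGameInstance; the hosting path is marked broken after a folder restructure.
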(event `Create Session`
  ; Create Session
  (`CreateSessionCallbackProxy.CreateSession` (`GameplayStatics.GetPlayerController` 0) 5
    (:`OnSuccess`
      (bind _returnvalue (`ColocationSetup.CreateByteArrayFromString` (`ColocationSetup.GetLocalIPAsString`)))
      (bind (_success _session) (`OculusXRAsyncAction_StartColocationSessionAdvertisement.OculusXRAsyncStartColocationSessionAdvertisement` _returnvalue)
        (:`OnComplete`
          (if _success
            ;; Fix this section. Broke from folder structure change
            (bind _asbp_colocation_session_game_instance (cast `/Game/Blueprints/ColocationSession/BP_ColocationSessionGameInstance` (`GameplayStatics.GetGameInstance`)))
            (set `/Game/Blueprints/ColocationSession/BP_ColocationSessionGameInstance.ColocationSession` _session _asbp_colocation_session_game_instance)
            (`GameplayStatics.OpenLevelBySoftObjectPtr` "/Game/Maps/BrickSpace.BrickSpace" true "?listen")))))))

(event `Find Sessions`
  ; Join Session
  (bind (_success _session) (`OculusXRAsyncAction_DiscoverColocationSessions.OculusXRAsyncDiscoverColocationSessions`)
    (:`SessionFound`
      (if _success
        (bind _asbp_colocation_session_game_instance (cast `/Game/Blueprints/ColocationSession/BP_ColocationSessionGameInstance` (`GameplayStatics.GetGameInstance`)))
        (bind _output_get (set `/Game/Blueprints/ColocationSession/BP_ColocationSessionGameInstance.ColocationSession` _session _asbp_colocation_session_game_instance))
        (`ColocationSetup.JoinColocationSession` _output_get)))))